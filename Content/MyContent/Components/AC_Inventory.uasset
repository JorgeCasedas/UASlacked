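; Inventory component that lets a character collect, combine, hold and use items, and creates the inventory, interact prompt and in-hand item widgets.
; Nearby interactables form a pool with a prompt on the first; interacting stores its inventory object and destroys the actor.
; Combining checks the selected object's CombinableWith class against the hovered one, replacing both with a constructed result.
; Held objects drive a hand mesh and widget image, and are removed when used.
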(event `self.ReceiveBeginPlay`
  (`|ExecutionSequence`
    (:`then_0`
      (bind _returnvalue (`|CreateWidget` "/Game/MyContent/Widgets/Inventory/WBP_Inventory.WBP_Inventory_C"))
      (bind _output_get (set `self.Inventory` _returnvalue))
      (`UserWidget.AddToViewport` _output_get 0))
    (:`then_1`
      (bind _returnvalue_2 (`|CreateWidget` "/Game/MyContent/Widgets/Interact/WBP_InteractPromp.WBP_InteractPromp_C"))
      (bind _output_get_2 (set `self.InteractPromp` _returnvalue_2))
      (`UserWidget.AddToViewport` _output_get_2 0)
      (`/Game/MyContent/Widgets/Interact/WBP_InteractPromp.Hide` _output_get_2))
    (:`then_2`
      (bind _returnvalue_3 (`|CreateWidget` "/Game/MyContent/Widgets/Inventory/WBP_InHandItem.WBP_InHandItem_C"))
      (bind _output_get_3 (set `self.InHandObjectWidget` _returnvalue_3))
      (`UserWidget.AddToViewport` _output_get_3 0)
      (`/Game/MyContent/Widgets/Inventory/WBP_InHandItem.SetHandObjectImage` _output_get_3 null))))

(event `InputAction|InventoryPrompTest`
  (params (Key :type "Key Structure"))
  (:`Pressed`
    (`/Game/MyContent/Widgets/Inventory/WBP_Inventory.ChangeState` (`self.Inventory`))))

(event `AddItem`
  (params (NewItem :type "/Game/MyContent/Objects/BP_InventoryObject Object Reference (by ref)"))
  (set `/Game/MyContent/Objects/BP_InventoryObject.InventoryComp` self NewItem)
  (`KismetArrayLibrary.Array_Add` (`self.Objects`) NewItem)
  (`/Game/MyContent/Widgets/Inventory/WBP_Inventory.FillInventory` (`self.Inventory`) (`self.Objects`)))

(event `RemoveItem`
  (params (ItemToRemove :type "/Game/MyContent/Objects/BP_InventoryObject Object Reference"))
  (`KismetArrayLibrary.Array_RemoveItem` (`self.Objects`) ItemToRemove)
  (`/Game/MyContent/Widgets/Inventory/WBP_Inventory.FillInventory` (`self.Inventory`) (`self.Objects`)))

(event `AddInteractableActorToPool`
  (params (NewItem :type "/Game/MyContent/Props/BP_InteractableObject Object Reference (by ref)"))
  (`KismetArrayLibrary.Array_Add` (`self.InteractActors`) NewItem)
  (`self.ShowPrompForInteractableObject`))

(event `RemoveInteractableActorFromPool`
  (params (Item :type "/Game/MyContent/Props/BP_InteractableObject Object Reference (by ref)"))
  (`KismetArrayLibrary.Array_RemoveItem` (`self.InteractActors`) Item)
  (`self.ShowPrompForInteractableObject`))

(event `ShowPrompForInteractableObject`
  (bind _interactactors (`self.InteractActors`))
  (if (> (`KismetArrayLibrary.Array_Length` _interactactors) 0)
    (`/Game/MyContent/Widgets/Interact/WBP_InteractPromp.Show` (`self.InteractPromp`) (`SceneComponent.K2_GetComponentLocation` (`/Game/MyContent/Props/BP_InteractableObject.PrompPosition` (`|GetArrayItem` _interactactors))))
    (else
      (`/Game/MyContent/Widgets/Interact/WBP_InteractPromp.Hide` (`self.InteractPromp`)))))

(event `GetActorIntoInventory`
  (bind _interactactors (`self.InteractActors`))
  (bind _output (`|GetArrayItem` _interactactors))
  (if (> (`KismetArrayLibrary.Array_Length` (`self.InteractActors`)) 0)
    (`self.AddItem` (`/Game/MyContent/Props/BP_InteractableObject.InventoryObject` _output))
    (set `self.LastInteractedActor` _output)
    (`KismetArrayLibrary.Array_Remove` _interactactors)
    (`self.ShowPrompForInteractableObject`)
    (`Actor.K2_DestroyActor` (`self.LastInteractedActor`))))

(event `EnhancedInput|/Game/ThirdPerson/Input/Actions/IA_Interact`
  (params (ActionValue :type Boolean) (ElapsedSeconds :type "Float (double-precision)") (TriggeredSeconds :type "Float (double-precision)") (InputAction :type "InputAction Object Reference" :default "/Game/ThirdPerson/Input/Actions/IA_Interact.IA_Interact"))
  (:`Triggered`
    (`self.GetActorIntoInventory`)))

(event `TryToCombineObjects`
  (params (Selected :type "/Game/MyContent/Objects/BP_InventoryObject Object Reference") (Hovered :type "/Game/MyContent/Objects/BP_InventoryObject Object Reference"))
  (bind _combinablewith (`/Game/MyContent/Objects/BP_InventoryObject.CombinableWith` Selected))
  (if (`KismetSystemLibrary.IsValidClass` _combinablewith)
    (if (== _combinablewith (`GameplayStatics.GetObjectClass` Hovered))
      (bind _returnvalue (`|GenericCreateObject` (`/Game/MyContent/Objects/BP_InventoryObject.CombinationResult` Selected)))
      (`self.AddItem` _returnvalue)
      (`self.RemoveItem` Selected)
      (`self.RemoveItem` Hovered))))

(event `SetObjectInCharacterHand`
  (params (Object :type "/Game/MyContent/Objects/BP_InventoryObject Object Reference"))
  (set `self.ObjectInHand` Object)
  (`StaticMeshComponent.SetStaticMesh` (`self.HandMeshComponent`) (`/Game/MyContent/Objects/BP_InventoryObject.ObjectMesh` Object))
  (`/Game/MyContent/Widgets/Inventory/WBP_InHandItem.SetHandObjectImage` (`self.InHandObjectWidget`) (`/Game/MyContent/Objects/BP_InventoryObject.Image` (`self.ObjectInHand`))))

(event `UnSetObjectInHand`
  (`StaticMeshComponent.SetStaticMesh` (`self.HandMeshComponent`) null)
  (`/Game/MyContent/Widgets/Inventory/WBP_InHandItem.SetHandObjectImage` (`self.InHandObjectWidget`) null))

(event `UseObjectInHand`
  (`self.UnSetObjectInHand`)
  (`self.RemoveItem` (`self.ObjectInHand`)))