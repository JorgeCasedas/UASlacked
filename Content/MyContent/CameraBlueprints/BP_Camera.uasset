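; Fixed-position level camera that takes over the view when the third-person character enters its CameraTrigger, or at BeginPlay if flagged as the first camera.
; The character tracks overlapped triggers, and the view blends back to it only when it leaves the last one.
; If following is enabled, a self-calling Delay loop rotates the camera toward the character, stopping only when that last-trigger exit clears CanRotate.
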(event `self.ReceiveBeginPlay`
  (if (`self.IsFirstCamera`)
    (`PlayerController.SetViewTargetWithBlend` (`GameplayStatics.GetPlayerController` 0) self 0.0 "VTBlend_Linear" 0.0 false)))

(event `self.CameraTrigger.OnActorBeginOverlap`
  (params (OverlappedActor :type "Actor Object Reference") (OtherActor :type "Actor Object Reference"))
  (bind _asbp_third_person_character (cast `/Game/ThirdPerson/Blueprints/BP_ThirdPersonCharacter` OtherActor))
  (`KismetArrayLibrary.Array_Add` (`/Game/ThirdPerson/Blueprints/BP_ThirdPersonCharacter.CameraTriggers` _asbp_third_person_character) (`self.CameraTrigger`))
  (`PlayerController.SetViewTargetWithBlend` (`GameplayStatics.GetPlayerController` 0) self 0.5 "VTBlend_Linear" 0.0 false)
  (if (`self.CanCameraFollow`)
    (set `self.CanRotate` true)
    (`self.RotateCamera`)))

(event `self.CameraTrigger.OnActorEndOverlap`
  (params (OverlappedActor :type "Actor Object Reference") (OtherActor :type "Actor Object Reference"))
  (bind _asbp_third_person_character (cast `/Game/ThirdPerson/Blueprints/BP_ThirdPersonCharacter` OtherActor))
  (bind _cameratriggers (`/Game/ThirdPerson/Blueprints/BP_ThirdPersonCharacter.CameraTriggers` _asbp_third_person_character))
  (`KismetArrayLibrary.Array_RemoveItem` _cameratriggers (`self.CameraTrigger`))
  (if (< (`KismetArrayLibrary.Array_Length` _cameratriggers) 1)
    (`PlayerController.SetViewTargetWithBlend` (`GameplayStatics.GetPlayerController` 0) _asbp_third_person_character 0.5 "VTBlend_Linear" 0.0 false)
    (set `self.CanRotate` false)))

(event `RotateCamera`
  (if (`self.CanRotate`)
    (`self.K2_SetActorRotation` (`KismetMathLibrary.FindLookAtRotation` (`self.K2_GetActorLocation`) (`self.K2_GetActorLocation` (stale `self.CameraTrigger.OnActorBeginOverlap` _asbp_third_person_character))))
    (`KismetSystemLibrary.Delay` 0.005)
    (`self.RotateCamera`)))

(fn `UserConstructionScript`)