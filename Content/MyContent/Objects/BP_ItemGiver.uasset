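; BP_ItemGiver is an interactable world object that gives the player a random inventory item.
; On BeginPlay it caches the AC_Inventory component from player pawn 0.
; InteractionBehaviour calls GiveItemToPlayer, which picks a random class from ItemsToGive and constructs it as an object.
; The object is cast to BP_InventoryObject and added to the cached inventory, with nothing added if the cast fails.
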(event `self.ReceiveBeginPlay`
  (set `self.InventoryComp` (`self.GetComponentByClass` (`GameplayStatics.GetPlayerPawn` 0) "/Game/MyContent/Components/AC_Inventory.AC_Inventory_C")))

(event `self.InteractionBehaviour`
  (`self.GiveItemToPlayer`))

(event `GiveItemToPlayer`
  (bind _itemstogive (`self.ItemsToGive`))
  (bind _returnvalue (`|GenericCreateObject` (`|GetArrayItem` _itemstogive (`KismetMathLibrary.RandomInteger` (`KismetArrayLibrary.Array_Length` _itemstogive)))))
  (bind _asbp_inventory_object (cast `/Game/MyContent/Objects/BP_InventoryObject` _returnvalue))
  (`/Game/MyContent/Components/AC_Inventory.AddItem` (`self.InventoryComp`) _asbp_inventory_object))

(fn `UserConstructionScript`)