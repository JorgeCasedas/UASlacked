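; BP_PickUpableObject is a prop the player can pick up, carry and drop.
; Its trigger overlap shows interact and pick-up prompt widgets and registers the actor in the player's AC_Interact pool.
; PickUp locks the interact component, disables mesh collision and attaches to the character's PickUpPivot.
; Drop detaches, unlocks, restores collision, line-traces down to place the object on the surface below, keeping only yaw, and both actions notify the interact component.
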(event `self.ReceiveBeginPlay`
  (bind _returnvalue (pcsubsystem `EnhancedInputLocalPlayerSubsystem` (`GameplayStatics.GetPlayerController` 0)))
  (`|ExecutionSequence`
    (:`then_0`
      (`/Engine/EditorBlueprintResources/StandardMacros.IsValid` _returnvalue
        (:`Is Valid`
          (`EnhancedInputSubsystemInterface.AddMappingContext` _returnvalue "/Game/ThirdPerson/Input/IMC_Default.IMC_Default" 0 (struct))
          (set `self.InteractComponent` (`self.GetComponentByClass` (`GameplayStatics.GetPlayerCharacter` 0) "/Game/MyContent/Components/AC_Interact.AC_Interact_C")))))
    (:`then_1`
      (bind _returnvalue_2 (`|CreateWidget` "/Game/MyContent/Widgets/Interact/WBP_InteractPromp.WBP_InteractPromp_C" null (`self.InteractPrompPivot`)))
      (bind _output_get (set `self.InteractPromp` _returnvalue_2))
      (`UserWidget.AddToViewport` _output_get 0)
      (bind _returnvalue_3 (`|CreateWidget` "/Game/MyContent/Widgets/Interact/WBP_PickUpPromp.WBP_PickUpPromp_C" null (`SceneComponent.K2_GetComponentLocation` (`self.PickUpPrompPivot`))))
      (bind _output_get_2 (set `self.PickUpPromp` _returnvalue_3))
      (`UserWidget.AddToViewport` _output_get_2 0))
    (:`then_2`
      (`self.HidePromps`))))

(event `self.Trigger.OnComponentBeginOverlap`
  (params (OverlappedComponent :type "PrimitiveComponent Object Reference") (OtherActor :type "Actor Object Reference") (OtherComp :type "PrimitiveComponent Object Reference") (OtherBodyIndex :type Integer) (bFromSweep :type Boolean) (SweepResult :type "HitResult Structure (by ref)"))
  (`/Game/MyContent/Widgets/Interact/WBP_InteractPromp.Show` (`self.InteractPromp`) (`self.InteractPrompPivot`))
  (`/Game/MyContent/Widgets/Interact/WBP_PickUpPromp.Show` (`self.PickUpPromp`) (`SceneComponent.K2_GetComponentLocation` (`self.PickUpPrompPivot`)))
  (`/Game/MyContent/Components/AC_Interact.AddInteractableActorToPool` (`self.InteractComponent`) self))

(event `self.Trigger.OnComponentEndOverlap`
  (params (OverlappedComponent :type "PrimitiveComponent Object Reference") (OtherActor :type "Actor Object Reference") (OtherComp :type "PrimitiveComponent Object Reference") (OtherBodyIndex :type Integer))
  (`self.HidePromps`)
  (`/Game/MyContent/Components/AC_Interact.RemoveInteractableActorFromPool` (`self.InteractComponent`) self))

(event `HidePromps`
  (`/Game/MyContent/Widgets/Interact/WBP_InteractPromp.Hide` (`self.InteractPromp`))
  (`/Game/MyContent/Widgets/Interact/WBP_PickUpPromp.Hide` (`self.PickUpPromp`)))

(event `PickUp`
  (set `/Game/MyContent/Components/AC_Interact.bLockObject` true (`self.InteractComponent`))
  (`PrimitiveComponent.SetCollisionEnabled` (`self.StaticMesh`) "NoCollision")
  (bind _asbp_third_person_character (cast `/Game/ThirdPerson/Blueprints/BP_ThirdPersonCharacter` (`GameplayStatics.GetPlayerCharacter` 0)))
  (`self.K2_AttachToComponent` (`/Game/ThirdPerson/Blueprints/BP_ThirdPersonCharacter.PickUpPivot` _asbp_third_person_character) "None" "SnapToTarget" "SnapToTarget" "KeepRelative")
  (`/Game/MyContent/Components/AC_Interact.OnPickUp` (`self.InteractComponent`)))

(event `Drop`
  (bind (_returnvalue_roll _returnvalue_pitch _returnvalue_yaw) (`KismetMathLibrary.BreakRotator` (`self.K2_GetActorRotation`)))
  (bind _returnvalue (`SceneComponent.K2_GetComponentLocation` (`self.StaticMesh`)))
  (`self.K2_DetachFromActor` "KeepWorld" "KeepWorld" "KeepWorld")
  (set `/Game/MyContent/Components/AC_Interact.bLockObject` false (`self.InteractComponent`))
  (`PrimitiveComponent.SetCollisionEnabled` (`self.StaticMesh`) "QueryAndPhysics")
  (bind _outhit (`KismetSystemLibrary.LineTraceSingleForObjects` _returnvalue (+ _returnvalue (* (0.0 0.0 1.0) -1000.0)) (`|MakeArray` "ObjectTypeQuery1" "ObjectTypeQuery2" :!type "EObjectTypeQuery Enum")))
  (`self.K2_SetActorLocation` (`.Location` (`GameplayStatics.BreakHitResult` _outhit)) true)
  (`/Game/MyContent/Components/AC_Interact.OnDrop` (`self.InteractComponent`))
  (`self.K2_SetActorRotation` (`KismetMathLibrary.MakeRotator` 0.0 0.0 _returnvalue_yaw)))

(fn `UserConstructionScript`)