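; Microwave prop that plays a sound on interaction and reacts specially to a spoon in hand.
; BeginPlay spawns a persistent, attenuated sound and stops it for reuse; Interact plays it if usable and not already playing.
; A spoon also disables further use and starts a short one-shot timer.
; An Explode event prints "Boom" and activates explosion and smoke, while ObjectSpecificAction alternates PickUp and Drop.
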(event `self.ReceiveBeginPlay`
  (`parent.ReceiveBeginPlay`)
  (bind _returnvalue (`GameplayStatics.SpawnSoundAtLocation` "/Game/MyContent/Sounds/microwave-92836.microwave-92836" (`self.K2_GetActorLocation`) (struct) 1.0 1.0 0.0 "/Game/MyContent/Sounds/SA_Main.SA_Main" null false))
  (bind _output_get (set `self.MicrowaveSound` _returnvalue))
  (`AudioComponent.Stop` _output_get))

(event `Explode`
  (`KismetSystemLibrary.PrintString` "Boom")
  (`ActorComponent.Activate` (`self.Explosion`) true)
  (`ActorComponent.Activate` (`self.Smoke`) true))

(event `/Game/MyContent/BPI_Interact.ObjectSpecificAction`
  (`/Engine/EditorBlueprintResources/StandardMacros.FlipFlop`
    (:`A`
      (`self.PickUp`))
    (:`B`
      (`self.Drop`))))

(fn `Interact`
  (params (HandObject :type "/Game/MyContent/Objects/BP_InventoryObject Object Reference"))
  (returns (ObjectsWhereCombined :type Boolean))
  (if (`self.bIsUsable`)
    (if (not (`AudioComponent.IsPlaying` (`self.MicrowaveSound`)))
      (`AudioComponent.Play` (`self.MicrowaveSound`) 0.0)
      (cast `/Game/MyContent/Objects/BP_Spoon` HandObject
        (:`then`
          (set `self.bIsUsable` false)
          (`KismetSystemLibrary.K2_SetTimerDelegate` (`|CreateDelegate` :!event `Explode`) 2.0)
          (return true))
        (:`CastFailed`
          (return false))))))

(fn `UserConstructionScript`
  (`parent.UserConstructionScript`))