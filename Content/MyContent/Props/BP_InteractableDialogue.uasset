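; BP_InteractableDialogue is a prop that plays multi-line dialogue for BP_ThirdPersonCharacterDialogueTest.
; Entering its box stores the character, shows a text prompt and creates a WBP_BaseDialogue widget; leaving hides both.
; EDialogue freezes movement, passes the Text array to the widget and advances its row, removing it and restoring movement at the last row.
; A DoOnce gates EDialogue but resets immediately after each step.
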(event `self.Box.OnComponentBeginOverlap`
  (params (OverlappedComponent :type "PrimitiveComponent Object Reference") (OtherActor :type "Actor Object Reference") (OtherComp :type "PrimitiveComponent Object Reference") (OtherBodyIndex :type Integer) (bFromSweep :type Boolean) (SweepResult :type "HitResult Structure (by ref)"))
  (bind _asbp_third_person_character_dialogue_test (cast `/Game/MyContent/TestBpStuff/BP_ThirdPersonCharacterDialogueTest` OtherActor))
  (set `self.As BP Third Person Character Dialogue Test` _asbp_third_person_character_dialogue_test)
  (`SceneComponent.SetHiddenInGame` (`self.TextRender`) false false)
  (bind _returnvalue (`|CreateWidget` "/Game/MyContent/Widgets/Dialogue/WBP_BaseDialogue.WBP_BaseDialogue_C"))
  (bind _output_get (set `self.DialogueWidget` _returnvalue))
  (`UserWidget.AddToViewport` _output_get 0))

(event `self.Box.OnComponentEndOverlap`
  (params (OverlappedComponent :type "PrimitiveComponent Object Reference") (OtherActor :type "Actor Object Reference") (OtherComp :type "PrimitiveComponent Object Reference") (OtherBodyIndex :type Integer))
  (bind _dialoguewidget (`self.DialogueWidget`))
  (cast `/Game/MyContent/TestBpStuff/BP_ThirdPersonCharacterDialogueTest` OtherActor)
  (`SceneComponent.SetHiddenInGame` (`self.TextRender`) true false)
  (`/Engine/EditorBlueprintResources/StandardMacros.IsValid` _dialoguewidget
    (:`Is Valid`
      (`Widget.RemoveFromParent` _dialoguewidget))))

(event `/Game/MyContent/Widgets/Dialogue/BI_Dialogue.E_Dialogue`
  (bind _dialoguewidget (`self.DialogueWidget`))
  (bind _dialoguewidget_2 (`self.DialogueWidget`))
  (bind _returnvalue (+ (`/Game/MyContent/Widgets/Dialogue/WBP_BaseDialogue.TextRow` _dialoguewidget_2) 1))
  (`/Engine/EditorBlueprintResources/StandardMacros.DoOnce` false :!label _label
    (:`Completed`
      (set `/Game/MyContent/TestBpStuff/BP_ThirdPersonCharacterDialogueTest.CanMove` false (`self.As BP Third Person Character Dialogue Test`))
      (set `/Game/MyContent/Widgets/Dialogue/WBP_BaseDialogue.Text` (`self.Text`) _dialoguewidget_2)
      (`Widget.SetVisibility` (`/Game/MyContent/Widgets/Dialogue/WBP_BaseDialogue.TextDialogue` _dialoguewidget_2) "Visible")
      (if (> _returnvalue (- (`KismetArrayLibrary.Array_Length` (`self.Text`)) 1))
        (`Widget.RemoveFromParent` _dialoguewidget)
        (set `/Game/MyContent/TestBpStuff/BP_ThirdPersonCharacterDialogueTest.CanMove` true (`self.As BP Third Person Character Dialogue Test`))
        (else
          (set `/Game/MyContent/Widgets/Dialogue/WBP_BaseDialogue.TextRow` _returnvalue _dialoguewidget)))
      (`self.resetDoOnce`))))

(event `resetDoOnce`
  (goto _label :!via `Reset`))

(fn `UserConstructionScript`)