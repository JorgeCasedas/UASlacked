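; BP_Door is an interactable door prop that responds according to what the player is holding.
; InteractionBehaviour checks the player's AC_Inventory ObjectInHand by casting it to BP_LoadedGun.
; With the loaded gun it only prints an "Exit the house" debug string, with no opening logic.
; Otherwise the third-person character says the locked-door line set on BeginPlay through SayDialogue.
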(event `self.ReceiveBeginPlay`
  (`parent.ReceiveBeginPlay`)
  (set `self.In Text` (`|MakeArray` "It is locked" :!type "Text")))

(event `self.InteractionBehaviour`
  (cast `/Game/MyContent/InventoryObjects/BP_LoadedGun` (`/Game/MyContent/Components/AC_Inventory.ObjectInHand` (`self.GetComponentByClass` (`GameplayStatics.GetPlayerCharacter` 0) "/Game/MyContent/Components/AC_Inventory.AC_Inventory_C"))
    (:`then`
      ;[1 1 1] Open door
      (`KismetSystemLibrary.PrintString` "Exit the house"))
    (:`CastFailed`
      ;[1 1 1] Make character say its a mirror
      (bind _asbp_third_person_character (cast `/Game/ThirdPerson/Blueprints/BP_ThirdPersonCharacter` (`GameplayStatics.GetPlayerCharacter` 0)))
      (`/Game/ThirdPerson/Blueprints/BP_ThirdPersonCharacter.SayDialogue` _asbp_third_person_character (`self.In Text`)))))

(fn `UserConstructionScript`
  (`parent.UserConstructionScript`))