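; BP_Mirror is an interactable mirror prop that reacts differently depending on what the player is holding.
; With a loaded gun in hand, interacting unlocks the "Soup Of Side" achievement and kills the player with a force originating from the held item's mesh location.
; Otherwise the player character comments on the mirror, and later interactions use a shorter, dismissive line.
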(event `self.ReceiveBeginPlay`
  (`parent.ReceiveBeginPlay`)
  (set `self.In Text` (`|MakeArray` "Hey, thats me!" "Well, obviously, it is a mirror" :!type "Text")))

(event `self.InteractionBehaviour`
  (cast `/Game/MyContent/InventoryObjects/BP_LoadedGun` (`/Game/MyContent/Components/AC_Inventory.ObjectInHand` (`self.GetComponentByClass` (`GameplayStatics.GetPlayerCharacter` 0) "/Game/MyContent/Components/AC_Inventory.AC_Inventory_C"))
    (:`then`
      ;[1 1 1] Soup of side
      (`KismetSystemLibrary.PrintString` "Die")
      (`/Game/AchievementSystem/Blueprints/Libraries/BP_AchievementsListLibrary.Unlock Achievement` "Soup Of Side")
      (bind _asbp_third_person_character (cast `/Game/ThirdPerson/Blueprints/BP_ThirdPersonCharacter` (`GameplayStatics.GetPlayerCharacter` 0)))
      (`/Game/ThirdPerson/Blueprints/BP_ThirdPersonCharacter.Die` _asbp_third_person_character 10000.0 (`SceneComponent.K2_GetComponentLocation` (`/Game/ThirdPerson/Blueprints/BP_ThirdPersonCharacter.MeshInHandComp` _asbp_third_person_character))))
    (:`CastFailed`
      ;[1 1 1] Make character say its a mirror
      (bind _asbp_third_person_character_2 (cast `/Game/ThirdPerson/Blueprints/BP_ThirdPersonCharacter` (`GameplayStatics.GetPlayerCharacter` 0)))
      (`/Game/ThirdPerson/Blueprints/BP_ThirdPersonCharacter.SayDialogue` _asbp_third_person_character_2 (`self.In Text`))
      (set `self.In Text` (`|MakeArray` "Yeah... mirror" :!type "Text")))))

(fn `UserConstructionScript`
  (`parent.UserConstructionScript`))