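; Clock prop that acts as the level's countdown and tells the player the time when interacted with.
; Tick adds elapsed seconds to a 21:20 start time and calls the third-person character's LoseGetCaught once the minutes pass 29.
; InteractionBehaviour has the character say the current time as dialogue, formatted HH:MM:SS through a zero-padding helper.
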(event `self.ReceiveBeginPlay`
  (`parent.ReceiveBeginPlay`)
  (set `self.InitialTime` (`KismetMathLibrary.MakeTimespan` 0 21 20)))

(event `self.ReceiveTick`
  (params (DeltaSeconds :type "Float (single-precision)"))
  (`parent.ReceiveTick` DeltaSeconds)
  (bind _output_get (set `self.TimeSeconds` (+ (`self.TimeSeconds`) DeltaSeconds)))
  (bind _output_get_2 (set `self.ActualTime` (+ (`self.InitialTime`) (`KismetMathLibrary.MakeTimespan` 0 0 0 (`KismetMathLibrary.FTrunc` _output_get)))))
  (if (> (`KismetMathLibrary.GetMinutes` _output_get_2) 29)
    (bind _asbp_third_person_character (cast `/Game/ThirdPerson/Blueprints/BP_ThirdPersonCharacter` (`GameplayStatics.GetPlayerCharacter` 0)))
    (`/Game/ThirdPerson/Blueprints/BP_ThirdPersonCharacter.LoseGetCaught` _asbp_third_person_character)))

(event `self.InteractionBehaviour`
  (bind _actualtime (`self.ActualTime`))
  (bind _asbp_third_person_character (cast `/Game/ThirdPerson/Blueprints/BP_ThirdPersonCharacter` (`GameplayStatics.GetPlayerCharacter` 0)))
  (`/Game/ThirdPerson/Blueprints/BP_ThirdPersonCharacter.SayDialogue` _asbp_third_person_character (`|MakeArray` (`KismetTextLibrary.Conv_StringToText` (`KismetStringLibrary.Concat_StrStr` (`self.TimeNumberToString` (`KismetMathLibrary.GetHours` _actualtime)) ":" (`self.TimeNumberToString` (`KismetMathLibrary.GetMinutes` _actualtime)) ":" (`self.TimeNumberToString` (`KismetMathLibrary.GetSeconds` _actualtime)))))))

(fn `TimeNumberToString`
  (params (TimeNumber :type Integer))
  (returns (TimeString :type String))
  (if (> TimeNumber 9)
    (return (`KismetStringLibrary.Conv_IntToString` TimeNumber))
    (else
      (return (`KismetStringLibrary.Concat_StrStr` "0" (`KismetStringLibrary.Conv_IntToString` TimeNumber))))))

(fn `UserConstructionScript`
  (`parent.UserConstructionScript`))