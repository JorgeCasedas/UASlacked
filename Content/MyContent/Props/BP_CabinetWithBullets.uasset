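; BP_CabinetWithBullets is an interactable cabinet prop that hands the player an item, presumably bullets, only once.
; InteractionBehaviour calls GiveItemToPlayer on first use and sets IsEmpty.
; Later interactions cast the player character to BP_ThirdPersonCharacter and call SayDialogue to report that nothing is left.
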(event `/Game/MyContent/Props/BP_InteractableObject.InteractionBehaviour`
  (if (`self.bIsEmpty`)
    ;[1 1 1] Make character say its empty
    (bind _asbp_third_person_character (cast `/Game/ThirdPerson/Blueprints/BP_ThirdPersonCharacter` (`GameplayStatics.GetPlayerCharacter` 0)))
    (`/Game/ThirdPerson/Blueprints/BP_ThirdPersonCharacter.SayDialogue` _asbp_third_person_character (`|MakeArray` "Nothing left here" :!type "Text"))
    (else
      (`self.GiveItemToPlayer`)
      (set `self.bIsEmpty` true))))

(fn `UserConstructionScript`
  (`parent.UserConstructionScript`))