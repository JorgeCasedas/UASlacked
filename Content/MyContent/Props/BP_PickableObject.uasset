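; BP_PickableObject is a prop that shows interact and pick-up prompts when its trigger is overlapped.
; On BeginPlay it adds the default Enhanced Input mapping context, then creates both prompt widgets at pivot components and hides them.
; Trigger overlap shows or hides the prompts and adds or removes the prop from the player character's AC_Interact pool.
; The PickUp event is an empty stub.
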(event `self.ReceiveBeginPlay`
  (bind _returnvalue (pcsubsystem `EnhancedInputLocalPlayerSubsystem` (`GameplayStatics.GetPlayerController` 0)))
  (`|ExecutionSequence`
    (:`then_0`
      (`/Engine/EditorBlueprintResources/StandardMacros.IsValid` _returnvalue
        (:`Is Valid`
          (`EnhancedInputSubsystemInterface.AddMappingContext` _returnvalue "/Game/ThirdPerson/Input/IMC_Default.IMC_Default" 0 (struct)))))
    (:`then_1`
      (bind _returnvalue_2 (`|CreateWidget` "/Game/MyContent/Widgets/Interact/WBP_InteractPromp.WBP_InteractPromp_C" null (`SceneComponent.K2_GetComponentLocation` (`self.InteractPrompPivot`))))
      (bind _output_get (set `self.InteractPromp` _returnvalue_2))
      (`UserWidget.AddToViewport` _output_get 0)
      (bind _returnvalue_3 (`|CreateWidget` "/Game/MyContent/Widgets/Interact/WBP_PickUpPromp.WBP_PickUpPromp_C" null (`SceneComponent.K2_GetComponentLocation` (`self.PickUpPrompPivot`))))
      (bind _output_get_2 (set `self.PickUpPromp` _returnvalue_3))
      (`UserWidget.AddToViewport` _output_get_2 0))
    (:`then_2`
      (`self.HidePromps`))))

(event `self.Trigger.OnComponentBeginOverlap`
  (params (OverlappedComponent :type "PrimitiveComponent Object Reference") (OtherActor :type "Actor Object Reference") (OtherComp :type "PrimitiveComponent Object Reference") (OtherBodyIndex :type Integer) (bFromSweep :type Boolean) (SweepResult :type "HitResult Structure (by ref)"))
  (`/Game/MyContent/Widgets/Interact/WBP_InteractPromp.Show` (`self.InteractPromp`) (`SceneComponent.K2_GetComponentLocation` (`self.InteractPrompPivot`)))
  (`/Game/MyContent/Widgets/Interact/WBP_PickUpPromp.Show` (`self.PickUpPromp`) (`SceneComponent.K2_GetComponentLocation` (`self.PickUpPrompPivot`)))
  (`/Game/MyContent/Components/AC_Interact.AddInteractableActorToPool` (`self.GetComponentByClass` (`GameplayStatics.GetPlayerCharacter` 0) "/Game/MyContent/Components/AC_Interact.AC_Interact_C") self))

(event `self.Trigger.OnComponentEndOverlap`
  (params (OverlappedComponent :type "PrimitiveComponent Object Reference") (OtherActor :type "Actor Object Reference") (OtherComp :type "PrimitiveComponent Object Reference") (OtherBodyIndex :type Integer))
  (`self.HidePromps`)
  (`/Game/MyContent/Components/AC_Interact.RemoveInteractableActorFromPool` (`self.GetComponentByClass` (`GameplayStatics.GetPlayerCharacter` 0) "/Game/MyContent/Components/AC_Interact.AC_Interact_C") self))

(event `HidePromps`
  (`/Game/MyContent/Widgets/Interact/WBP_InteractPromp.Hide` (`self.InteractPromp`))
  (`/Game/MyContent/Widgets/Interact/WBP_PickUpPromp.Hide` (`self.PickUpPromp`)))

(event `PickUp`)

(fn `UserConstructionScript`)